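; AI pawn that follows the player's DDCharacter and carries health and AI state widgets.
; BeginPlay caches the player, starts the follow loop and sets itself as Owner on both widgets.
; FollowPlayer re-checks every half second, moving toward the player beyond PlayerOffset, otherwise targeting itself to halt.
; StopFollowingPlayer enters that halt branch, which still feeds the loop, so following resumes after the delay.
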(event `self.ReceiveBeginPlay`
  (bind _asddcharacter (cast `DDCharacter` (`GameplayStatics.GetPlayerCharacter` 0)))
  (set `self.Player` _asddcharacter)
  (`self.Follow Player`)
  (bind _aswb_health (cast `/Game/Blueprints/Widgets/WB_Health` (`WidgetComponent.GetWidget` (`self.HealthWidget`))))
  (set `/Game/Blueprints/Widgets/WB_Health.Owner` self _aswb_health)
  (bind _aswb_aistate (cast `/Game/Blueprints/Widgets/WB_AIState` (`WidgetComponent.GetWidget` (`self.AIStateWidget`))))
  (set `/Game/Blueprints/Widgets/WB_AIState.Owner` self _aswb_aistate))

(event `Follow Player`
  ;[1 1 1] Simple AI system of following the player
  (if (> (`self.GetDistanceTo` (`self.Player`)) (`self.PlayerOffset`))
    (`|AIMoveTo` self (0.0 0.0 0.0) (`self.Player`)
      (:`then`
        _))
    (else
      (`|AIMoveTo` self (0.0 0.0 0.0) self :!label _label
        (:`then`
          _))))
  (`KismetSystemLibrary.Delay` 0.5)
  (`self.Follow Player`))

(event `Stop Following Player`
  ;[1 1 1] Simple AI system of following the player
  (goto _label))

(fn `UserConstructionScript`)