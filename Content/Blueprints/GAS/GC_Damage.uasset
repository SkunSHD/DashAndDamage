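; Damage gameplay cue that checks whether the hit DDGASBaseCharacter target has died.
; On execute it reads a float attribute, presumably health, from the target's ability system component.
; At zero or below it prints a "play death montage" debug string as a placeholder and calls the parent OnExecute.
; If the attribute is missing or still positive, it returns false without calling the parent.
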(fn `OnExecute`
  (params (MyTarget :type "Actor Object Reference") (Parameters :type "GameplayCueParameters Structure (by ref)"))
  (returns (ReturnValue :type Boolean))
  (bind _asddgasbase_character (cast `DDGASBaseCharacter` MyTarget))
  (bind (_bsuccessfullyfoundattribute _returnvalue) (`AbilitySystemBlueprintLibrary.GetFloatAttributeFromAbilitySystemComponent` (`AbilitySystemBlueprintLibrary.GetAbilitySystemComponent` _asddgasbase_character) (struct :`AttributeName` "Health" :`Attribute` "/Script/DD.DDAttributeSet:Health")))
  (if _bsuccessfullyfoundattribute
    (if (<= _returnvalue 0.0)
      (`KismetSystemLibrary.PrintString` null "play death montage")
      (return (`parent.OnExecute` MyTarget Parameters))
      (else
        (return false)))
    (else
      (return false))))