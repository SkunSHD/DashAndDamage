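; BP_AI is an AI pawn that follows the player's DDCharacter and carries health and AI-state widgets.
; BeginPlay caches the player, starts following, and links both widgets to itself.
; FollowPlayer re-runs every half second, moving to the player beyond PlayerOffset and otherwise targeting itself to halt.
; StopFollowingPlayer enters that halt branch, which still re-enters the follow loop after the delay.
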(event `self.ReceiveBeginPlay`
  ;[1 1 1] Make UI Follow The Player
  (bind _returnvalue (`GameplayStatics.GetActorOfClass` "/Script/DD.DDCharacter"))
  (set `self.Player` _returnvalue)
  (`self.Follow Player`)
  ;[1 1 1] Init widgets
  (`/Game/Blueprints/Widgets/WB_Health.Initialize` (cast `/Game/Blueprints/Widgets/WB_Health` (`WidgetComponent.GetWidget` (`self.HealthWidget`)) :!pure true) self)
  (set `/Game/Blueprints/Widgets/WB_AIState.Owner` self (cast `/Game/Blueprints/Widgets/WB_AIState` (`WidgetComponent.GetWidget` (`self.AIStateWidget`)) :!pure true)))

(event `Follow Player`
  ;[1 1 1] Simple AI system of following the player
  (if (> (`self.GetDistanceTo` (`self.Player`)) (`self.PlayerOffset`))
    (`|AIMoveTo` self (0.0 0.0 0.0) (`self.Player`)
      (:`then`
        _))
    (else
      (`|AIMoveTo` self (0.0 0.0 0.0) self :!label _label
        (:`then`
          _))))
  (`KismetSystemLibrary.Delay` 0.5)
  (`self.Follow Player`))

(event `Stop Following Player`
  ;[1 1 1] Simple AI system of following the player
  (goto _label))

(fn `UserConstructionScript`)